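; Enemy actor that chases the player, deals contact damage to BP_Diver and awards score on death.
; Every tick it issues an eased MoveComponentTo toward the player's X/Y, with rotation derived from its spawn location and PlayerLocation, which is never set here.
; Capsule overlap damages the diver; incoming damage lowers Health until it adds score to BP_Round and destroys itself.
; Roam-radius and interpolation logic is left unused.
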(event `self.ReceiveTick`
  (params (DeltaSeconds :type "Float (single-precision)"))
  (`self.Attack`))

(event `self.ReceiveBeginPlay`
  ;[1 1 1] On Play
  (set `self.CurrentLocation` (`self.K2_GetActorLocation`)))

(event `Attack`
  (bind (_returnvalue_x _returnvalue_y) (`KismetMathLibrary.BreakVector` (`self.K2_GetActorLocation` (`GameplayStatics.GetPlayerCharacter` 0))))
  ;[1 1 1] Move to player
  (bind _output_get (set `self.DistanceX` _returnvalue_x))
  (bind _output_get_2 (set `self.DistanceY` _returnvalue_y))
  (`KismetSystemLibrary.MoveComponentTo` (`self.DefaultSceneRoot`) (`KismetMathLibrary.MakeVector` _output_get _output_get_2) (`KismetMathLibrary.FindLookAtRotation` (`self.CurrentLocation`) (`self.PlayerLocation`)) false true))

(event `self.ReceiveAnyDamage`
  (params (Damage :type "Float (single-precision)") (DamageType :type "DamageType Object Reference") (InstigatedBy :type "Controller Object Reference") (DamageCauser :type "Actor Object Reference"))
  ;[1 1 1] Get damaged
  (bind _output_get (set `self.Health` (- (`self.Health`) Damage)))
  (if (<= _output_get 0.0)
    (bind _returnvalue (`GameplayStatics.GetActorOfClass` "/Game/Chi/Round/BP_Round.BP_Round_C"))
    (`/Game/Chi/Round/BP_Round.IncreaseScore` _returnvalue 1000.0)
    (`self.K2_DestroyActor`)))

(event `self.CapsuleCollision.OnComponentBeginOverlap`
  (params (OverlappedComponent :type "PrimitiveComponent Object Reference") (OtherActor :type "Actor Object Reference") (OtherComp :type "PrimitiveComponent Object Reference") (OtherBodyIndex :type Integer) (bFromSweep :type Boolean) (SweepResult :type "HitResult Structure (by ref)"))
  ;[1 1 1] Damage player
  (bind _asbp_diver (cast `/Game/Chi/Diver/BP_Diver` OtherActor))
  (`GameplayStatics.ApplyDamage` _asbp_diver (`self.Damage`) null self))

(fn `UserConstructionScript`)