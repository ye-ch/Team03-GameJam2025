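; BP_Enemy is an enemy that chases the player and damages the diver on contact.
; Every Tick calls Attack, which uses an eased MoveComponentTo to send the root toward the player character's X and Y, without feeding in Z.
; A capsule overlap with BP_Diver applies the Damage value.
; Roam-radius checks and interpolated movement are left disconnected, and MoveCloser is an empty stub.
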(event `MoveCloser`)

(event `self.ReceiveBeginPlay`
  (set `self.CurrentLocation` (`self.K2_GetActorLocation`)))

(event `self.ReceiveTick`
  (params (DeltaSeconds :type "Float (single-precision)"))
  (`self.Attack`))

(event `self.Capsule.OnComponentBeginOverlap`
  (params (OverlappedComponent :type "PrimitiveComponent Object Reference") (OtherActor :type "Actor Object Reference") (OtherComp :type "PrimitiveComponent Object Reference") (OtherBodyIndex :type Integer) (bFromSweep :type Boolean) (SweepResult :type "HitResult Structure (by ref)"))
  (bind _asbp_diver (cast `/Game/Chi/Diver/BP_Diver` OtherActor))
  (`GameplayStatics.ApplyDamage` _asbp_diver (`self.Damage`) null self))

(event `Attack`
  (bind (_returnvalue_x _returnvalue_y) (`KismetMathLibrary.BreakVector` (`self.K2_GetActorLocation` (`GameplayStatics.GetPlayerCharacter` 0))))
  (bind _output_get (set `self.DistanceX` _returnvalue_x))
  (bind _output_get_2 (set `self.DistanceY` _returnvalue_y))
  (`KismetSystemLibrary.MoveComponentTo` (`self.DefaultSceneRoot`) (`KismetMathLibrary.MakeVector` _output_get _output_get_2) (struct) false true))

(fn `UserConstructionScript`)