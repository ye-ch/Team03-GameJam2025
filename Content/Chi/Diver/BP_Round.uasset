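; BP_Round is a round countdown timer that flags when the round is over.
; The construction script fills CurrentTime from MaxTime, and Tick caches DeltaSeconds.
; SubtractTime, which nothing live in this Blueprint starts, re-schedules itself each tick to subtract that delta, then clamps at zero, clears the timer and sets IsRoundEnd.
; GetTimePercentage returns the remaining fraction of the round.
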(event `self.ReceiveBeginPlay`)

(event `self.ReceiveTick`
  (params (DeltaSeconds :type "Float (single-precision)"))
  (bind _output_get (set `self.Delta Seconds` DeltaSeconds)))

(event `SubtractTime`
  (bind _returnvalue (`KismetSystemLibrary.K2_SetTimerForNextTickDelegate` (delegate `SubtractTime`)))
  (set `self.RoundTimerHandler` _returnvalue)
  (bind _output_get (set `self.CurrentTime` (- (`self.CurrentTime`) (`self.Delta Seconds`))))
  (if (<= _output_get 0.0)
    (set `self.CurrentTime` 0.0)
    (`KismetSystemLibrary.K2_ClearAndInvalidateTimerHandle` (`self.RoundTimerHandler`))
    (set `self.IsRoundEnd` true)))

(fn `GetTimePercentage`
  (returns (Percentage :type "Float (double-precision)"))
  (return (/ (`self.CurrentTime`) (`self.MaxTime`))))

(fn `UserConstructionScript`
  (set `self.CurrentTime` (`self.MaxTime`)))