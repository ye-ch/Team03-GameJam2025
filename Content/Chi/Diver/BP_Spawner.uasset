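; BP_Spawner is an actor Blueprint in the Diver folder that, despite its name, contains no spawning logic yet.
; Its event graph and construction script are empty, and nothing in the file calls its one helper.
; PolarToCartesian turns Theta and Phi in degrees into X, Y, Z components without a radius.
; X uses Sin(Theta) where standard spherical conversion uses Sin(Phi), so results deviate from the unit sphere.
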(fn `PolarToCartesian`
  (params (Theta :type "Float (double-precision)") (Phi :type "Float (double-precision)"))
  (returns (x :type "Float (double-precision)") (y :type "Float (double-precision)") (z :type "Float (double-precision)"))
  (bind _returnvalue (`KismetMathLibrary.DegreesToRadians` (`local.Phi`)))
  (bind _returnvalue_2 (`KismetMathLibrary.DegreesToRadians` (`local.Theta`)))
  (bind _returnvalue_3 (`KismetMathLibrary.Sin` _returnvalue_2))
  (return (* (`KismetMathLibrary.Cos` _returnvalue_2) _returnvalue_3) (* _returnvalue_3 (`KismetMathLibrary.Sin` _returnvalue)) (`KismetMathLibrary.Cos` _returnvalue)))

(fn `UserConstructionScript`)