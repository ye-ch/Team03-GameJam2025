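; BP_Spawner is a spawner meant to place BP_Cube actors at random points on a sphere around the world origin.
; A looping one-second timer fires SpawnEnemy, but that event is empty and the Spawn logic is disconnected, so nothing spawns.
; The unwired logic converts random spherical angles through PolarToCartesian and scales by Radius, with MaxAngle trimming both polar caps.
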(event `self.ReceiveBeginPlay`
  (`KismetSystemLibrary.K2_SetTimerDelegate` (delegate `SpawnEnemy`) 1.0 true))

(event `SpawnEnemy`)

(fn `PolarToCartesian`
  (params (Theta :type "Float (double-precision)") (Phi :type "Float (double-precision)"))
  (returns (Coords :type "Vector Structure"))
  (bind _returnvalue (`KismetMathLibrary.DegreesToRadians` (`local.Phi`)))
  (bind _returnvalue_2 (`KismetMathLibrary.DegreesToRadians` (`local.Theta`)))
  (bind _returnvalue_3 (`KismetMathLibrary.Sin` _returnvalue_2))
  (return (`KismetMathLibrary.MakeVector` (* _returnvalue_3 (`KismetMathLibrary.Cos` _returnvalue)) (* _returnvalue_3 (`KismetMathLibrary.Sin` _returnvalue)) (`KismetMathLibrary.Cos` _returnvalue_2))))

(fn `Spawn`)

(fn `UserConstructionScript`)