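; BP_Round manages a timed round, tracking remaining time and score and pushing score updates to the BP_Diver's HUD.
; After a two-second delay, a self-rescheduling timer counts time down by the cached frame delta, and GetTimePercentage exposes the fraction left.
; At zero, EndRound folds current score into the total, resets it, clears BP_Spawner's timer and destroys all BP_Enemy actors.
; BeginRound is an empty stub.
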(event `self.ReceiveBeginPlay`
  (`|ExecutionSequence`
    (:`then_0`
      (bind _asbp_diver (cast `/Game/Chi/Diver/BP_Diver` (`GameplayStatics.GetPlayerCharacter` 0)))
      (set `self.Diver` _asbp_diver))
    (:`then_1`
      (`KismetSystemLibrary.K2_SetTimerDelegate` (delegate `SubtractTime`) 2.0))))

(event `SubtractTime`
  (bind _output_get (set `self.CurrentTime` (- (`self.CurrentTime`) (`self.Delta Seconds`))))
  (`KismetSystemLibrary.K2_SetTimerDelegate` (delegate `SubtractTime`) (`self.Delta Seconds`))
  (set `self.TimerHandler` (struct))
  (if (<= _output_get 0.0)
    (set `self.CurrentTime` 0.0)
    (set `self.IsRoundEnd` true)
    (`self.EndRound`)))

(event `self.ReceiveTick`
  (params (DeltaSeconds :type "Float (single-precision)"))
  (set `self.Delta Seconds` DeltaSeconds))

(fn `BeginRound`)

(fn `EndRound`
  (set `self.TotalScore` (+ (`self.TotalScore`) (`self.CurrentScore`)))
  (bind _output_get (set `self.CurrentScore` 0.0))
  (`/Game/Chi/UI/WBP_HUD.UpdateScore` (`/Game/Chi/Diver/BP_Diver.HUD` (`self.Diver`)) _output_get)
  (bind _returnvalue (`GameplayStatics.GetActorOfClass` "/Game/Chi/Round/BP_Spawner.BP_Spawner_C"))
  (`KismetSystemLibrary.K2_ClearAndInvalidateTimerHandle` (`/Game/Chi/Round/BP_Spawner.TimerHandler` _returnvalue))
  (bind _outactors (`GameplayStatics.GetAllActorsOfClass` "/Game/Chen/Enemy/BP_Enemy.BP_Enemy_C"))
  (for _array_element _outactors
    (`self.K2_DestroyActor` _array_element)
    (`KismetSystemLibrary.K2_ClearAndInvalidateTimerHandle` (`self.TimerHandler`))))

(fn `GetTimePercentage`
  (returns (Percentage :type "Float (double-precision)"))
  (return (/ (`self.CurrentTime`) (`self.MaxTime`))))

(fn `IncreaseScore`
  (params (Score :type "Float (double-precision)"))
  (bind _output_get (set `self.TotalScore` (+ Score (`self.TotalScore`))))
  (`/Game/Chi/UI/WBP_HUD.UpdateScore` (`/Game/Chi/Diver/BP_Diver.HUD` (`self.Diver`)) _output_get))

(fn `UserConstructionScript`
  (set `self.CurrentTime` (`self.MaxTime`)))